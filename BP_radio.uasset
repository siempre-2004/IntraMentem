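; BP_radio is an interactable radio prop that toggles its audio on and off.
; It starts with audio paused and its widget hidden; the interact event (IBPE交互) calls 播放, which flips the 正在播放 flag to either pause playback or unpause and restart it from the beginning.
; The highlight event (IBP高亮显示) drives the mesh's custom depth rendering and the widget's visibility together.
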(event `self.ReceiveBeginPlay`
  (`AudioComponent.SetPaused` (`self.Audio`) true)
  (`SceneComponent.SetVisibility` (`self.Widget`) false true))

(event `播放`
  (bind _audio (`self.Audio`))
  (if (`self.正在播放`)
    (`AudioComponent.SetPaused` _audio true)
    (set `self.正在播放` false)
    (else
      (`AudioComponent.SetPaused` _audio false)
      (`AudioComponent.Play` _audio 0.0)
      (set `self.正在播放` true))))

(event `高亮显示`
  (params (`高亮显示` :type Boolean))
  (`PrimitiveComponent.SetRenderCustomDepth` (`self.StaticMesh`) `高亮显示`)
  (`SceneComponent.SetVisibility` (`self.Widget`) `高亮显示` true))

(event `/Game/BP/IBP_交互接口.IBP_E交互`
  (`self.播放`))

(event `/Game/BP/IBP_交互接口.IBP_高亮显示`
  (params (`高亮显示` :type Boolean))
  (`self.高亮显示` `高亮显示`))

(fn `UserConstructionScript`)