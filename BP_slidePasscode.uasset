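; Sliding passcode lock puzzle with four clickable sliders, each stepping through positions 1 to 4.
; A click, ignored while a slider moves, updates that slider's stored position and direction via F更新移动方向与位置, reversing at either end.
; 移动 then animates its relative Z by a signed step with a shared Timeline Lerp.
; On finish, F_更新解锁状态 compares all positions against 正确位置信息 and calls the 解锁完成 dispatcher on a match.
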(event `self.StaticMesh1.OnClicked`
  (params (TouchedComponent :type "PrimitiveComponent Object Reference") (ButtonPressed :type "Key Structure"))
  (if (not (`self.正在移动`))
    (bind (`_更新后的位置` `_更新后的方向`) (`self.F 更新移动方向与位置` (`self.1号位置`) (`self.1号位置向下移动`)))
    (set `self.1号位置` `_更新后的位置`)
    (set `self.1号位置向下移动` `_更新后的方向`)
    (`self.移动` (`self.StaticMesh1`) (`self.1号位置向下移动`))))

(event `self.StaticMesh2.OnClicked`
  (params (TouchedComponent :type "PrimitiveComponent Object Reference") (ButtonPressed :type "Key Structure"))
  (if (not (`self.正在移动`))
    (bind (`_更新后的位置` `_更新后的方向`) (`self.F 更新移动方向与位置` (`self.2号位置`) (`self.2号位置向下移动`)))
    (set `self.2号位置` `_更新后的位置`)
    (set `self.2号位置向下移动` `_更新后的方向`)
    (`self.移动` (`self.StaticMesh2`) (`self.2号位置向下移动`))))

(event `self.StaticMesh3.OnClicked`
  (params (TouchedComponent :type "PrimitiveComponent Object Reference") (ButtonPressed :type "Key Structure"))
  (if (not (`self.正在移动`))
    (bind (`_更新后的位置` `_更新后的方向`) (`self.F 更新移动方向与位置` (`self.3号位置`) (`self.3号位置向下移动`)))
    (set `self.3号位置` `_更新后的位置`)
    (set `self.3号位置向下移动` `_更新后的方向`)
    (`self.移动` (`self.StaticMesh3`) (`self.3号位置向下移动`))))

(event `self.StaticMesh4.OnClicked`
  (params (TouchedComponent :type "PrimitiveComponent Object Reference") (ButtonPressed :type "Key Structure"))
  (if (not (`self.正在移动`))
    (bind (`_更新后的位置` `_更新后的方向`) (`self.F 更新移动方向与位置` (`self.4号位置`) (`self.4号位置向下移动`)))
    (set `self.4号位置` `_更新后的位置`)
    (set `self.4号位置向下移动` `_更新后的方向`)
    (`self.移动` (`self.StaticMesh4`) (`self.4号位置向下移动`))))

(event `移动`
  (params (`滑块` :type "StaticMeshComponent Object Reference") (`向下移动` :type Boolean))
  (bind `_初始高度位置` (`self.初始高度位置`))
  (bind (`_相对位置_x` `_相对位置_y`) (`KismetMathLibrary.BreakVector` (`self.相对位置`)))
  (bind _returnvalue (`KismetMathLibrary.Abs` (`self.移动位置差`)))
  (set `self.正在移动` true)
  (bind _output_get (set `self.相对位置` (`SceneComponent.RelativeLocation` `滑块`)))
  (set `self.初始高度位置` (.z _output_get))
  (if `向下移动`
    (set `self.移动位置差` (* _returnvalue -1.0))
    (bind (_direction `_新建轨道_0`) (`Timeline|时间轴_0` :!via `PlayFromStart` :!label _label)
      (:`Update`
        (`SceneComponent.K2_SetRelativeLocation` `滑块` (`KismetMathLibrary.MakeVector` `_相对位置_x` `_相对位置_y` (`KismetMathLibrary.Lerp` `_初始高度位置` (+ `_初始高度位置` (`self.移动位置差`)) `_新建轨道_0`)) false false))
      (:`Finished`
        (`self.F_更新解锁状态`)
        (set `self.正在移动` false)
        (set `self.移动位置差` (`KismetMathLibrary.Abs` (`self.移动位置差`)))))
    (else
      (set `self.移动位置差` _returnvalue)
      (goto _label :!via `PlayFromStart`))))

(fn `F 更新移动方向与位置`
  (params (`当前位置` :type Integer) (`当前方向` :type Boolean))
  (returns (`更新后的位置` :type Integer) (`更新后的方向` :type Boolean))
  (locals (`L_当前方向` :type Boolean) (`L_当前位置` :type Integer))
  (bind _returnvalue (+ `当前位置` (select `bool` (`local.L_当前方向`) :`false` -1 :`true` 1)))
  (set `local.L_当前位置` `当前位置`)
  (set `local.L_当前方向` `当前方向`)
  (if (or (> _returnvalue 4) (< _returnvalue 1))
    (if (> (+ (`local.L_当前位置`) (select `bool` (`local.L_当前方向`) :`false` -1 :`true` 1)) 4)
      (set `local.L_当前位置` 3)
      (set `local.L_当前方向` (not (`local.L_当前方向`)))
      (else
        (set `local.L_当前位置` 2)
        (set `local.L_当前方向` (not (`local.L_当前方向`)))))
    (else
      (set `local.L_当前位置` (+ (`local.L_当前位置`) (select `bool` (`local.L_当前方向`) :`false` -1 :`true` 1)))))
  (return (`local.L_当前位置`) (`local.L_当前方向`)))

(fn `F_更新解锁状态`
  (locals (`L_密码正确` :type Boolean :default true))
  (if (and (== (`|GetArrayItem` (`self.正确位置信息`)) (`self.1号位置`)) (== (`|GetArrayItem` (`self.正确位置信息`) 1) (`self.2号位置`)) (== (`|GetArrayItem` (`self.正确位置信息`) 2) (`self.3号位置`)) (== (`|GetArrayItem` (`self.正确位置信息`) 3) (`self.4号位置`)))
    (`self.ED_解锁完成`)
    (return)
    (else
      (return))))

(fn `UserConstructionScript`)