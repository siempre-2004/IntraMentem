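; Interactable box whose door opens only when the player carries a key item.
; On interaction it searches the player pawn's backpack component for the key, removes it, then a timeline swings the door open and marks it opened.
; Without a key it shows a no-key prompt widget, throttled by a short delay.
; Interface-driven highlighting toggles custom depth and a widget until the box is opened.
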(event `self.ReceiveBeginPlay`
  (`SceneComponent.SetVisibility` (`self.Widget`) false true))

(event `高亮显示`
  (params (`高亮显示` :type Boolean))
  (`PrimitiveComponent.SetRenderCustomDepth` (`self.StaticMesh1`) `高亮显示`)
  (`SceneComponent.SetVisibility` (`self.Widget`) `高亮显示` true))

(event `/Game/BP/IBP_交互接口.IBP_高亮显示`
  (params (`高亮显示` :type Boolean))
  (if (not (`self.已开启`))
    (`self.高亮显示` `高亮显示`)))

(event `/Game/BP/IBP_交互接口.IBP_E交互`
  (`self.F_判断玩家是否有钥匙`)
  (if (`self.可开门`)
    (`/Engine/EditorBlueprintResources/StandardMacros.DoOnce` false
      (:`Completed`
        (bind (_direction `_新建轨道_0`) (`Timeline|时间轴_0`)
          (:`Update`
            (`SceneComponent.K2_SetRelativeRotation` (`self.开启门`) (`KismetMathLibrary.MakeRotator` 0.0 0.0 (`KismetMathLibrary.Lerp` 0.0 -90.0 `_新建轨道_0`)) false false))
          (:`Finished`
            (set `self.已开启` true)))))
    (elif (`self.可触发提示`)
      (bind _returnvalue (`|CreateWidget` "/Game/BP/钥匙开启的盒子/无钥匙提示.无钥匙提示_C"))
      (`UserWidget.AddToViewport` _returnvalue 0)
      (set `self.可触发提示` false)
      (`KismetSystemLibrary.Delay` 1.0)
      (set `self.可触发提示` true))))

(event `/Game/BP/IBP_交互接口.IBP_F交互`)

(fn `F_判断玩家是否有钥匙`
  (for (_array_element _array_index) (`/Game/BP/背包系统/CBP_背包.物品栏` (`self.GetComponentByClass` (`GameplayStatics.GetPlayerPawn` 0) "/Game/BP/背包系统/CBP_背包.CBP_背包_C"))
    (if (== (`.ActorClass_7_0A372B7841DE3D0A8FA3619F30EEDA30` (break `/Game/BP/背包系统/S_物品信息` _array_element)) "/Game/BP/背包系统/BP_可拾取物品_钥匙.BP_可拾取物品_钥匙_C")
      (set `self.可开门` true)
      (`/Game/BP/背包系统/CBP_背包.删除物品` (`self.GetComponentByClass` (`GameplayStatics.GetPlayerPawn` 0) "/Game/BP/背包系统/CBP_背包.CBP_背包_C") _array_index)
      (break)))
  (return))

(fn `UserConstructionScript`)