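; Interactable safe that stays locked until its child sliding code-bar puzzle (BP_滑动密码条) fires its unlock event.
; Unlocking automatically swings the door open once via a Timeline yaw rotation, then marks it opened.
; Interacting while locked shows a "cannot open" hint widget, throttled by a one-second delay.
; Interface-driven highlighting toggles custom depth and a prompt widget until the safe is opened.
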(event `self.ReceiveBeginPlay`
  (`SceneComponent.SetVisibility` (`self.Widget`) false true)
  (bind `_asbp_滑动密码条` (cast `/Game/BP/滑动密码盒子/BP_滑动密码条` (`ChildActorComponent.ChildActor` (`self.ChildActor`))))
  (add `/Game/BP/滑动密码盒子/BP_滑动密码条.ED_解锁完成` `_asbp_滑动密码条` (delegate `开启`)))

(event `开启`
  (set `self.可开门` true)
  (`self.IBP_E交互`))

(event `高亮显示`
  (params (`高亮显示` :type Boolean))
  (`PrimitiveComponent.SetRenderCustomDepth` (`self.StaticMesh1`) `高亮显示`)
  (`SceneComponent.SetVisibility` (`self.Widget`) `高亮显示` true))

(event `/Game/BP/IBP_交互接口.IBP_高亮显示`
  (params (`高亮显示` :type Boolean))
  (if (not (`self.已开启`))
    (`self.高亮显示` `高亮显示`)))

(event `/Game/BP/IBP_交互接口.IBP_E交互`
  (if (`self.可开门`)
    (`/Engine/EditorBlueprintResources/StandardMacros.DoOnce` false
      (:`Completed`
        (bind (_direction `_新建轨道_0`) (`Timeline|时间轴_0`)
          (:`Update`
            (`SceneComponent.K2_SetRelativeRotation` (`self.开启门`) (`KismetMathLibrary.MakeRotator` 0.0 0.0 (`KismetMathLibrary.Lerp` 0.0 -90.0 `_新建轨道_0`)) false false))
          (:`Finished`
            (set `self.已开启` true)
            (`self.高亮显示` false)))))
    (elif (`self.可触发提示`)
      (bind _returnvalue (`|CreateWidget` "/Game/BP/滑动密码盒子/WBP_不可开保险箱提示.WBP_不可开保险箱提示_C"))
      (`UserWidget.AddToViewport` _returnvalue 0)
      (set `self.可触发提示` false)
      (`KismetSystemLibrary.Delay` 1.0)
      (set `self.可触发提示` true))))

(fn `UserConstructionScript`)