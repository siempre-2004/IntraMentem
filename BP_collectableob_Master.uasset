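; Master Blueprint for collectable world objects that can be highlighted, picked up into the player's backpack and switched to physics.
; BeginPlay hides the prompt widget and records the actor's own class in its item-info struct.
; Interface events toggle custom-depth highlight with the widget, or pass the struct to the player pawn's CBP_背包 component on E-interact, destroying the actor if accepted.
; 开启重力 enables gravity and physics simulation on the mesh.
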(event `self.ReceiveBeginPlay`
  (`SceneComponent.SetVisibility` (`self.Widget`) false true)
  (bind _structout (setmembers `/Game/BP/背包系统/S_物品信息` :`StructRef` (`self.S_物品信息`) :`ActorClass` (`GameplayStatics.GetObjectClass` self)))
  (set `self.S_物品信息` _structout))

(event `高亮显示`
  (params (`高亮显示` :type Boolean))
  (`PrimitiveComponent.SetRenderCustomDepth` (`self.StaticMesh`) `高亮显示`)
  (`SceneComponent.SetVisibility` (`self.Widget`) `高亮显示` true))

(event `触发拾取`
  (bind `_已拿起` (`/Game/BP/背包系统/CBP_背包.F_拿起物品` (`self.GetComponentByClass` (`GameplayStatics.GetPlayerPawn` 0) "/Game/BP/背包系统/CBP_背包.CBP_背包_C") (`self.S_物品信息`)))
  (if `_已拿起`
    (`self.K2_DestroyActor`)))

(event `/Game/BP/IBP_交互接口.IBP_高亮显示`
  (params (`高亮显示` :type Boolean))
  (`self.高亮显示` `高亮显示`))

(event `/Game/BP/IBP_交互接口.IBP_E交互`
  (`self.触发拾取`))

(event `/Game/BP/IBP_交互接口.IBP_F交互`)

(event `开启重力`
  (bind _staticmesh (`self.StaticMesh`))
  (`PrimitiveComponent.SetEnableGravity` _staticmesh true)
  (`PrimitiveComponent.SetSimulatePhysics` _staticmesh true))

(fn `UserConstructionScript`)