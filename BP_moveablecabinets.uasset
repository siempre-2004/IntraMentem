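; Interactable sliding cabinet or drawer that toggles between open and closed.
; Highlight interface event toggles custom depth on the mesh and a prompt widget, which starts hidden.
; Interact event runs a timeline that lerps the whole actor along the Arrow's forward axis, reversing direction by open state.
; DoOnce gates block retriggering mid-move; on finish it flips the state, fires the open-drawer dispatcher and resets them.
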(event `self.ReceiveBeginPlay`
  (`SceneComponent.SetVisibility` (`self.Widget`) false true))

(event `高亮显示`
  (params (`高亮显示` :type Boolean))
  (`PrimitiveComponent.SetRenderCustomDepth` (`self.StaticMesh`) `高亮显示`)
  (`SceneComponent.SetVisibility` (`self.Widget`) `高亮显示` true))

(event `/Game/BP/IBP_交互接口.IBP_高亮显示`
  (params (`高亮显示` :type Boolean))
  (`self.高亮显示` `高亮显示`))

(event `/Game/BP/IBP_交互接口.IBP_E交互`
  (bind `_初始位置` (`self.初始位置`))
  (if (`self.已开启`)
    (`/Engine/EditorBlueprintResources/StandardMacros.DoOnce` false :!label _label
      (:`Completed`
        (set `self.初始位置` (`self.K2_GetActorLocation` self))
        (bind (_direction `_新建轨道_0`) (`Timeline|时间轴_0` :!via `PlayFromStart` :!label _label_2)
          (:`Update`
            (`self.K2_SetActorLocation` self (`KismetMathLibrary.VLerp` `_初始位置` (+ `_初始位置` (* (`SceneComponent.GetForwardVector` (`self.Arrow`)) (select `bool` (`self.已开启`) :`false` 40 :`true` -40))) `_新建轨道_0`) false false))
          (:`Finished`
            (bind _output_get (set `self.已开启` (not (`self.已开启`))))
            (`self.ED_开启抽屉` _output_get)
            (`|ExecutionSequence`
              (:`then_0`
                (goto _label :!via `Reset`))
              (:`then_1`
                (goto _label_3 :!via `Reset`)))))))
    (else
      (`/Engine/EditorBlueprintResources/StandardMacros.DoOnce` false :!label _label_3
        (:`Completed`
          (set `self.初始位置` (`self.K2_GetActorLocation`))
          (goto _label_2 :!via `PlayFromStart`))))))

(fn `UserConstructionScript`)