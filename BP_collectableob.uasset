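; BP_collectableob is an interactable item actor that shows its description in a note-viewer widget when interacted with.
; The interact interface event creates WBP_查看纸条 from the item struct's intro text only if none is open, then clears the reference through its close dispatcher.
; A highlight event toggles custom depth on the mesh and two prompt widgets, hidden at BeginPlay.
; A separate event turns on mesh physics simulation.
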(event `self.ReceiveBeginPlay`
  (`parent.ReceiveBeginPlay`)
  (`SceneComponent.SetVisibility` (`self.Widget`) false true)
  (`SceneComponent.SetVisibility` (`self.Widget1`) false true))

(event `/Game/BP/IBP_交互接口.IBP_F交互`
  (`self.WBP_查看纸条`
    (:`then`)
    (:`else`
      (bind _returnvalue (`|CreateWidget` "/Game/BP/背包系统/WBP_查看纸条.WBP_查看纸条_C" null (`.介绍_11_B1768242467C0E2E92A7159048AE05CC` (break `/Game/BP/背包系统/S_物品信息` (`self.S_物品信息`)))))
      (bind _output_get (set `self.WBP_查看纸条` _returnvalue))
      (`UserWidget.AddToViewport` _output_get 0)
      (add `/Game/BP/背包系统/WBP_查看纸条.ED_点击关闭` _output_get (delegate `关闭查看`)))))

(event `关闭查看`
  (set `self.WBP_查看纸条` null))

(event `self.高亮显示`
  (params (`高亮显示` :type Boolean))
  (`PrimitiveComponent.SetRenderCustomDepth` (`self.StaticMesh`) `高亮显示`)
  (`SceneComponent.SetVisibility` (`self.Widget`) `高亮显示` true)
  (`SceneComponent.SetVisibility` (`self.Widget1`) `高亮显示` true))

(event `开启重力`
  (`PrimitiveComponent.SetSimulatePhysics` (`self.StaticMesh`) true))

(fn `UserConstructionScript`
  (`parent.UserConstructionScript`))