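; BP_slidelock is an interactable password lock that opens a code-entry puzzle UI and reports success.
; Interface-driven highlighting toggles the mesh's custom depth and a prompt widget, which starts hidden.
; Interacting creates the password widget from the actor's password struct, unless one is already valid, and binds its correct and wrong events.
; Both results clear the widget reference, and a correct code also fires the lock's password-correct dispatcher.
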(event `self.ReceiveBeginPlay`
  (`SceneComponent.SetVisibility` (`self.Widget`) false true))

(event `高亮显示`
  (params (`高亮显示` :type Boolean))
  (`PrimitiveComponent.SetRenderCustomDepth` (`self.StaticMesh`) `高亮显示`)
  (`SceneComponent.SetVisibility` (`self.Widget`) `高亮显示` true))

(event `/Game/BP/IBP_交互接口.IBP_高亮显示`
  (params (`高亮显示` :type Boolean))
  (`self.高亮显示` `高亮显示`))

(event `/Game/BP/IBP_交互接口.IBP_E交互`
  (`self.WBP_数字密码锁`
    (:`then`)
    (:`else`
      (bind _returnvalue (`|CreateWidget` "/Game/BP/数字密码锁/解密_数字密码输入面板/UI_解密_密码输入.UI_解密_密码输入_C" null (`self.密码结构体`)))
      (bind _output_get (set `self.WBP_数字密码锁` _returnvalue))
      (`UserWidget.AddToViewport` _output_get 0)
      (add `/Game/BP/数字密码锁/解密_数字密码输入面板/UI_解密_密码输入.ED_密码正确` _output_get (delegate `密码正确`))
      (add `/Game/BP/数字密码锁/解密_数字密码输入面板/UI_解密_密码输入.ED_密码错误` _output_get (delegate `密码错误`)))))

(event `密码错误`
  (set `self.WBP_数字密码锁` null))

(event `密码正确`
  (set `self.WBP_数字密码锁` null)
  (`self.ED_密码正确`))

(fn `UserConstructionScript`)