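; A password-locked door actor that opens on interaction once its linked lock reports a correct password.
; At BeginPlay it binds to the lock's password-correct dispatcher (密码正确), which sets the openable flag.
; Interacting then plays a one-shot Timeline rotating the door 90 degrees in yaw, or otherwise shows a cannot-open widget with a one-second cooldown.
; An interface highlight event toggles custom depth and a prompt widget until the door has finished opening.
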(event `self.ReceiveBeginPlay`
  (`SceneComponent.SetVisibility` (`self.Widget`) false true)
  (bind `_密码锁` (`self.密码锁`)
    (:`then`
      (add `/Game/BP/数字密码锁/BP_数字密码锁.ED_密码正确` `_密码锁` (delegate `设置为可开门`)))
    (:`else`)))

(event `设置为可开门`
  (set `self.可开门` true))

(event `高亮显示`
  (params (`高亮显示` :type Boolean))
  (`PrimitiveComponent.SetRenderCustomDepth` (`self.StaticMesh`) `高亮显示`)
  (`SceneComponent.SetVisibility` (`self.Widget`) `高亮显示` true))

(event `/Game/BP/IBP_交互接口.IBP_高亮显示`
  (params (`高亮显示` :type Boolean))
  (if (not (`self.已开启`))
    (`self.高亮显示` `高亮显示`)))

(event `/Game/BP/IBP_交互接口.IBP_E交互`
  (if (`self.可开门`)
    (`/Engine/EditorBlueprintResources/StandardMacros.DoOnce` false
      (:`Completed`
        (bind (_direction `_新建轨道_0`) (`Timeline|时间轴_0`)
          (:`Update`
            (`SceneComponent.K2_SetRelativeRotation` (`self.Scene`) (`KismetMathLibrary.MakeRotator` 0.0 0.0 (`KismetMathLibrary.Lerp` 0.0 90.0 `_新建轨道_0`)) false false))
          (:`Finished`
            (set `self.已开启` true)))))
    (elif (`self.可触发提示`)
      (bind _returnvalue (`|CreateWidget` "/Game/BP/数字密码锁/WBP_不可开门提示.WBP_不可开门提示_C"))
      (`UserWidget.AddToViewport` _returnvalue 0)
      (set `self.可触发提示` false)
      (`KismetSystemLibrary.Delay` 1.0)
      (set `self.可触发提示` true))))

(fn `UserConstructionScript`)