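; BP_4X4cabinet is a puzzle cabinet that slides aside to reveal a passage once all its designated correct drawers are open.
; On BeginPlay it binds to each listed drawer's open event dispatcher and caches its starting location.
; Each opening triggers a check across that list; when it passes, a timeline lerps the cabinet 300 units along its Arrow's forward vector.
; An end-game call on the first-person character is left unconnected.
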(event `self.ReceiveBeginPlay`
  (for _array_element (`self.指定正确的抽屉`)
    (add `/Game/BP/抽屉/BP_可移动抽屉.ED_开启抽屉` _array_element (delegate `移开_露出通道`))
    (set `self.初始位置` (`self.K2_GetActorLocation` self))))

(event `移开_露出通道`
  (params (`已开启` :type Boolean))
  (bind `_初始位置` (`self.初始位置`))
  (if `已开启`
    (bind `_可开启` (`self.f-判断是否可以开启`))
    (if `_可开启`
      (bind (_direction `_新建轨道_0`) (`Timeline|时间轴_0`)
        (:`Update`
          (`self.K2_SetActorLocation` self (`KismetMathLibrary.VLerp` `_初始位置` (+ `_初始位置` (* (`SceneComponent.GetForwardVector` (`self.Arrow`)) 300)) `_新建轨道_0`) false false))))))

(fn `f-判断是否可以开启`
  (returns (`可开启` :type Boolean))
  (locals (`L-可开启` :type Boolean :default true))
  (for _array_element (`self.指定正确的抽屉`)
    (if (not (`/Game/BP/抽屉/BP_可移动抽屉.已开启` _array_element))
      (set `local.L-可开启` false)
      (break)))
  (return (`local.L-可开启`)))

(fn `UserConstructionScript`)