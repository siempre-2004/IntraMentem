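; Final door actor that ends the game when the player interacts with it.
; The interact interface event casts the player pawn to FirstPersonCharacter and calls its 结束游戏 (end game) function.
; The highlight interface event toggles the mesh's custom depth and the prompt widget's visibility, both switched off at BeginPlay.
; A FlipFlop timeline that would swing the door 90 degrees is left disconnected and never runs.
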(event `self.ReceiveBeginPlay`
  (`self.高亮显示` false))

(event `self.IBP_E交互`
  (bind _asfirst_person_character (cast `/Game/FirstPersonBP/Blueprints/FirstPersonCharacter` (`GameplayStatics.GetPlayerPawn` 0)))
  (`/Game/FirstPersonBP/Blueprints/FirstPersonCharacter.结束游戏` _asfirst_person_character))

(event `self.IBP_高亮显示`
  (params (`高亮显示` :type Boolean))
  (`self.高亮显示` `高亮显示`))

(event `高亮显示`
  (params (`高亮显示` :type Boolean))
  (`PrimitiveComponent.SetRenderCustomDepth` (`self.StaticMesh`) `高亮显示`)
  (`SceneComponent.SetVisibility` (`self.Widget`) `高亮显示` true))

(fn `UserConstructionScript`)